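; Spawn_Cube_BP is a cube obstacle that starts hidden without collision and appears after a random delay once the game starts.
; StartGame or the Enter key feeds a DoOnce that triggers this first appearance.
; When the cube hits an actor with "Wall" in its name, it hides, waits a random delay, then returns to its saved start location and reappears.
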(event `self.ReceiveBeginPlay`
  (set `self.start location` (`SceneComponent.K2_GetComponentLocation` (`self.Cube`)))
  (`self.SetActorEnableCollision` false)
  (`self.SetActorHiddenInGame` true))

(event `StartGame`
  (`/Engine/EditorBlueprintResources/StandardMacros.DoOnce` false :!label _label
    (:`Completed`
      (`KismetSystemLibrary.Delay` (`KismetMathLibrary.RandomFloatInRange` 5.0 10.0))
      (`self.SetActorEnableCollision` true)
      (`self.SetActorHiddenInGame` false))))

(event `Key|Enter`
  (params (Key :type "Key Structure"))
  (:`Pressed`
    (goto _label)))

(event `self.ReceiveTick`
  (params (DeltaSeconds :type "Float (single-precision)")))

(event `self.Cube.OnComponentHit`
  (params (HitComponent :type "PrimitiveComponent Object Reference") (OtherActor :type "Actor Object Reference") (OtherComp :type "PrimitiveComponent Object Reference") (NormalImpulse :type "Vector Structure") (Hit :type "HitResult Structure (by ref)"))
  (if (`KismetStringLibrary.Contains` (`KismetSystemLibrary.GetObjectName` OtherActor) "Wall")
    (`self.SetActorEnableCollision` false)
    (`self.SetActorHiddenInGame` true)
    (`KismetSystemLibrary.Delay` (`KismetMathLibrary.RandomFloatInRange` 1.0 10.0))
    (`SceneComponent.K2_SetWorldLocationAndRotation` :`self` (`self.Cube`) :`NewLocation` (`self.start location`) :`bSweep` true :`bTeleport` true)
    (`self.SetActorEnableCollision` true)
    (`self.SetActorHiddenInGame` false)))

(fn `UserConstructionScript`)