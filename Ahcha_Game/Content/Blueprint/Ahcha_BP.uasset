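; Player character Blueprint that moves along fixed world axes, with debug keys to open a test level and switch camera.
; Direction buttons and a D-pad, decoded by float tolerance into right, down and left, add movement input; right and left also drive accelerate/brake flags.
; Tick updates airborne and ground-proximity flags via movement state and a capsule trace, clearing the Button2 jump flag.
; Analog-stick movement is left disconnected.
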(event `StartCharMove`
  (`ActorComponent.SetActive` (`self.CharacterMovement`) true true))

(event `self.ReceiveTick`
  (params (DeltaSeconds :type "Float (single-precision)"))
  (`self.Check_Dpad_Zero`)
  (`self.IsFalling`))

(event `EnhancedInput|/Game/Input/inputs/LeftY`
  (params (ActionValue :type "Float (double-precision)") (ElapsedSeconds :type "Float (double-precision)") (TriggeredSeconds :type "Float (double-precision)") (InputAction :type "InputAction Object Reference" :default "/Game/Input/inputs/LeftY.LeftY"))
  ;[1 1 1] Comment
  (:`Triggered`
    (set `self.Left Y Value` ActionValue)))

(event `Update_Movement`
  ;[1 1 1] Comment
  (`|ExecutionSequence`))

(event `Key|R`
  (params (Key :type "Key Structure"))
  (:`Pressed`
    (`GameplayStatics.OpenLevel` "Cenario_teste" false)))

(event `Key|Two`
  (params (Key :type "Key Structure"))
  ;[1 1 1] Camera
  (:`Pressed`
    (`PlayerController.SetViewTargetWithBlend` (`GameplayStatics.GetPlayerController` 0) (`ActorComponent.GetOwner` (`self.Camera`)) 0.0 "VTBlend_Linear" 0.0 false)))

(event `EnhancedInput|/Game/Input/inputs/LeftX`
  (params (ActionValue :type "Float (double-precision)") (ElapsedSeconds :type "Float (double-precision)") (TriggeredSeconds :type "Float (double-precision)") (InputAction :type "InputAction Object Reference" :default "/Game/Input/inputs/LeftX.LeftX"))
  ;[1 1 1] Comment
  (:`Triggered`
    (set `self.Left X Value` ActionValue)))

(event `EnhancedInput|/Game/Input/inputs/DPad`
  (params (ActionValue :type "Float (double-precision)") (ElapsedSeconds :type "Float (double-precision)") (TriggeredSeconds :type "Float (double-precision)") (InputAction :type "InputAction Object Reference" :default "/Game/Input/inputs/DPad.DPad"))
  ;[1 1 1] Comment
  (:`Triggered`
    (set `self.Dpad Value` ActionValue :!label _label)
    (`KismetSystemLibrary.PrintString` (`KismetStringLibrary.Concat_StrStr` "Dpad Value: " (`KismetStringLibrary.Conv_DoubleToString` ActionValue)))
    (`self.Dpad Right`)
    (`self.Dpad Down`)
    (`self.Dpad Left`))
  (:`Completed`
    (goto _label)))

(event `EnhancedInput|/Game/Input/inputs/Button4`
  (params (ActionValue :type Boolean) (ElapsedSeconds :type "Float (double-precision)") (TriggeredSeconds :type "Float (double-precision)") (InputAction :type "InputAction Object Reference" :default "/Game/Input/inputs/Button4.Button4"))
  ;[1 1 1] Comment
)

(event `EnhancedInput|/Game/Input/inputs/ButtonUp`
  (params (ActionValue :type Boolean) (ElapsedSeconds :type "Float (double-precision)") (TriggeredSeconds :type "Float (double-precision)") (InputAction :type "InputAction Object Reference" :default "/Game/Input/inputs/ButtonUp.ButtonUp"))
  ;[1 1 1] Comment
  (:`Triggered`
    (`self.AddMovementInput` (5.0 0.0 0.0) 1.0 true)))

(event `EnhancedInput|/Game/Input/inputs/Button1`
  (params (ActionValue :type Boolean) (ElapsedSeconds :type "Float (double-precision)") (TriggeredSeconds :type "Float (double-precision)") (InputAction :type "InputAction Object Reference" :default "/Game/Input/inputs/Button1.Button1"))
  ;[1 1 1] Comment
)

(event `Check_Dpad_Zero`
  ;[1 1 1] Comment
  (if (`KismetMathLibrary.NearlyEqual_FloatFloat` 0.0 0.0 0.15)
    _))

(event `EnhancedInput|/Game/Input/inputs/Button3`
  (params (ActionValue :type Boolean) (ElapsedSeconds :type "Float (double-precision)") (TriggeredSeconds :type "Float (double-precision)") (InputAction :type "InputAction Object Reference" :default "/Game/Input/inputs/Button3.Button3"))
  ;[1 1 1] Comment
)

(event `EnhancedInput|/Game/Input/inputs/ButtonRight`
  (params (ActionValue :type Boolean) (ElapsedSeconds :type "Float (double-precision)") (TriggeredSeconds :type "Float (double-precision)") (InputAction :type "InputAction Object Reference" :default "/Game/Input/inputs/ButtonRight.ButtonRight"))
  ;[1 1 1] Comment
  (:`Triggered`
    (`self.AddMovementInput` (0.0 5.0 0.0) 1.0 true :!label _label_2)
    (set `self.IsAceel` true))
  (:`Completed`
    (set `self.IsAceel` false)))

(event `Jump_Impulse`
  ;[1 1 1] Comment
  (`self.Jump`))

(event `EnhancedInput|/Game/Input/inputs/ButtonLeft`
  (params (ActionValue :type Boolean) (ElapsedSeconds :type "Float (double-precision)") (TriggeredSeconds :type "Float (double-precision)") (InputAction :type "InputAction Object Reference" :default "/Game/Input/inputs/ButtonLeft.ButtonLeft"))
  ;[1 1 1] Comment
  (:`Triggered`
    (`self.AddMovementInput` (0.0 -5.0 0.0) 1.0 true :!label _label_3)
    (set `self.isBreak` true))
  (:`Completed`
    (set `self.isBreak` false)))

(event `EnhancedInput|/Game/Input/inputs/Button2`
  (params (ActionValue :type Boolean) (ElapsedSeconds :type "Float (double-precision)") (TriggeredSeconds :type "Float (double-precision)") (InputAction :type "InputAction Object Reference" :default "/Game/Input/inputs/Button2.Button2"))
  ;[1 1 1] Comment
  (:`Triggered`
    (set `self.isJump` true)))

(event `Dpad Left`
  ;[1 1 1] Comment
  (if (`KismetMathLibrary.NearlyEqual_FloatFloat` (`self.Dpad Value`) 0.85 0.15)
    (goto _label_3)))

(event `Dpad Right`
  ;[1 1 1] Comment
  (if (`KismetMathLibrary.NearlyEqual_FloatFloat` (`self.Dpad Value`) 0.28 0.15)
    (goto _label_2)))

(event `self.ReceiveHit`
  (params (MyComp :type "PrimitiveComponent Object Reference") (Other :type "Actor Object Reference") (OtherComp :type "PrimitiveComponent Object Reference") (bSelfMoved :type Boolean) (HitLocation :type "Vector Structure") (HitNormal :type "Vector Structure") (NormalImpulse :type "Vector Structure") (Hit :type "HitResult Structure (by ref)"))
  ;[1 1 1] Comment
  (if (not (`KismetMathLibrary.Conv_IntToBool` (`KismetStringLibrary.FindSubstring` (`KismetSystemLibrary.GetDisplayName` Other) "Esteira")))
    _
    (else
      _))
  (set `self.isJump` false))

(event `IsFalling`
  (bind _x (.x (`SceneComponent.K2_GetComponentLocation` (`self.Mesh`))))
  (bind _y (.y (`SceneComponent.K2_GetComponentLocation` (`self.Mesh`))))
  ;[1 1 1] Comment
  (if (`NavMovementComponent.IsFalling` (`self.CharacterMovement`))
    (set `self.inAir` true)
    (else
      (set `self.inAir` false)))
  (`|ExecutionSequence`
    (:`then_1`
      (bind (_outhit _returnvalue) (`KismetSystemLibrary.CapsuleTraceSingle` (`KismetMathLibrary.MakeVector` _x _y) (`KismetMathLibrary.MakeVector` _x _y (- (.z (`SceneComponent.K2_GetComponentLocation` (`self.Mesh`))) 50.0)) 50.0 0.0 "TraceTypeQuery1"))
      (if _returnvalue
        (set `self.IsGroundNear` true)
        (else
          (set `self.IsGroundNear` false)))
      (set `self.isJump` false))))

(event `EnhancedInput|/Game/Input/inputs/ButtonDown`
  (params (ActionValue :type Boolean) (ElapsedSeconds :type "Float (double-precision)") (TriggeredSeconds :type "Float (double-precision)") (InputAction :type "InputAction Object Reference" :default "/Game/Input/inputs/ButtonDown.ButtonDown"))
  ;[1 1 1] Comment
  (:`Triggered`
    (`self.AddMovementInput` (-5.0 0.0 0.0) 1.0 true :!label _label_4)))

(event `Dpad Down`
  ;[1 1 1] Comment
  (if (`KismetMathLibrary.NearlyEqual_FloatFloat` (`self.Dpad Value`) 0.57 0.15)
    (goto _label_4)))

(fn `UserConstructionScript`)