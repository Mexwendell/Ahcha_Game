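; Conveyor belt or tread (esteira) Blueprint whose shape the player character can adjust during play.
; The construction script tiles mesh segments along a spline, spaced by mesh X bounds.
; A timeline slides the segments along the spline, wrapping negative distances by spline length.
; Tick reads Ahcha_Character_BP to move one spline point vertically, clamped to a BeginPlay minimum height, and adjusts segment spacing to match.
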(event `self.ReceiveBeginPlay`
  (`self.Play_Esteira`)
  (set `self.EixoWPos` (`SceneComponent.K2_GetComponentLocation` (`self.StaticMesh`)))
  (set `self.SplinePointLocation` (`SplineComponent.GetLocationAtSplinePoint` (`self.Spline`) (`self.Point Index`) "World")))

(event `Play_Esteira`
  (bind _spline (`self.Spline`))
  (bind _distancealongspline (`self.DistanceAlongSpline`))
  (bind _staticmesharray (`self.StaticMeshArray`))
  (bind (_direction _newtrack_0) (`Timeline|Timeline` :`NewTime` 1.0 :!via `PlayFromStart`)
    (:`Update`
      (set `self.Timeline_value` _newtrack_0)
      (for (_array_element _array_index) _staticmesharray
        (bind _output_get (set `self.DistanceAlongSpline` (- (* (- (`KismetArrayLibrary.Array_Length` _staticmesharray) _array_index) (`self.Xlenght`)) (`KismetMathLibrary.Lerp` 0.0 (`SplineComponent.GetSplineLength` (`self.Spline`)) _newtrack_0))))
        (if (< _output_get 0.0)
          (set `self.DistanceAlongSpline` (+ (`SplineComponent.GetSplineLength` (`self.Spline`)) (`self.DistanceAlongSpline`))))
        (`SceneComponent.K2_SetRelativeLocationAndRotation` _array_element (`SplineComponent.GetLocationAtDistanceAlongSpline` _spline _distancealongspline "Local") (`SplineComponent.GetRotationAtDistanceAlongSpline` _spline _distancealongspline "Local") false false)))))

(event `self.ReceiveTick`
  (params (DeltaSeconds :type "Float (single-precision)"))
  (bind _spline (`self.Spline`))
  (bind _point_index (`self.Point Index`))
  (bind (_returnvalue_x _returnvalue_y _returnvalue_z) (`KismetMathLibrary.BreakVector` (+ (`SplineComponent.GetLocationAtSplinePoint` _spline _point_index "World") (`KismetMathLibrary.MakeVector` 0.0 0.0 (`self.Esteira Control`)))))
  (bind _asahcha_character_bp (cast `/Game/Blueprint/Ahcha_Character_BP` (`GameplayStatics.GetPlayerCharacter` 0)))
  (set `self.Point Index` (`/Game/Blueprint/Ahcha_Character_BP.SplinePointNum` _asahcha_character_bp))
  (set `self.Esteira Control` (`/Game/Blueprint/Ahcha_Character_BP.Esteira_control` _asahcha_character_bp))
  (`SplineComponent.SetLocationAtSplinePoint` _spline _point_index (`KismetMathLibrary.MakeVector` _returnvalue_x _returnvalue_y (`KismetMathLibrary.FMax` _returnvalue_z (.z (`self.SplinePointLocation`)))) "World" true)
  (set `self.Xlenght` (+ (`self.Xlenght`) (/ (`self.Esteira Control`) (- (`KismetArrayLibrary.Array_Length` (`self.StaticMeshArray`)) 1)))))

(fn `UserConstructionScript`
  (bind _spline (`self.Spline`))
  (bind (_returnvalue_min _returnvalue_max) (break `Box` (`StaticMesh.GetBoundingBox` (`self.Mesh`))))
  (bind _returnvalue_x (`KismetMathLibrary.BreakVector` (+ (`KismetMathLibrary.Vector_GetAbs` _returnvalue_min) (`KismetMathLibrary.Vector_GetAbs` _returnvalue_max))))
  (bind _output_get (set `self.Xlenght` _returnvalue_x))
  (for _index (range (`KismetMathLibrary.FTrunc` (/ (`SplineComponent.GetSplineLength` (`self.Spline`)) _output_get)))
    (bind _returnvalue (* _index (`self.Xlenght`)))
    (bind _returnvalue_2 (`AddComponent|NODE_AddStaticMeshComponent-0` :`RelativeTransform` (`KismetMathLibrary.MakeTransform` (`SplineComponent.GetLocationAtDistanceAlongSpline` _spline _returnvalue "Local") (`SplineComponent.GetRotationAtDistanceAlongSpline` _spline _returnvalue "Local"))))
    (`StaticMeshComponent.SetStaticMesh` _returnvalue_2 (`self.Mesh`))
    (`KismetArrayLibrary.Array_Add` (`self.StaticMeshArray`) _returnvalue_2)))