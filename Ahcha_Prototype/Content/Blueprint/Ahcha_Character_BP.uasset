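; Player character Blueprint that maps a gamepad's raw sticks, D-pad and buttons to fixed world-axis movement and a jump.
; Tick polls left-stick values against 0.25/0.75 thresholds and checks for a near-zero D-pad value as forward.
; The D-pad is a single float, decoded into other directions by tolerance bands on input events.
; Keyboard keys set and print a spline point number and EsteiraControl (conveyor) value, or switch the view target.
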(event `EnhancedInput|/Game/Input/inputs/DPad`
  (params (ActionValue :type "Float (double-precision)") (ElapsedSeconds :type "Float (double-precision)") (TriggeredSeconds :type "Float (double-precision)") (InputAction :type "InputAction Object Reference" :default "/Game/Input/inputs/DPad.DPad"))
  ;[1 1 1] Comment
  (:`Triggered`
    (set `self.Dpad_Value` ActionValue :!label _label)
    (`self.DpadRight`)
    (`self.DpadDown`)
    (`self.DpadLeft`))
  (:`Completed`
    (goto _label)))

(event `EnhancedInput|/Game/Input/inputs/ButtonUp`
  (params (ActionValue :type Boolean) (ElapsedSeconds :type "Float (double-precision)") (TriggeredSeconds :type "Float (double-precision)") (InputAction :type "InputAction Object Reference" :default "/Game/Input/inputs/ButtonUp.ButtonUp"))
  ;[1 1 1] Comment
  (:`Triggered`
    (`self.AddMovementInput` (5.0 0.0 0.0) :!label _label_2)))

(event `EnhancedInput|/Game/Input/inputs/Button4`
  (params (ActionValue :type Boolean) (ElapsedSeconds :type "Float (double-precision)") (TriggeredSeconds :type "Float (double-precision)") (InputAction :type "InputAction Object Reference" :default "/Game/Input/inputs/Button4.Button4"))
  ;[1 1 1] Comment
)

(event `Check_Dpad_Zero`
  ;[1 1 1] Comment
  (if (`KismetMathLibrary.NearlyEqual_FloatFloat` (`self.Dpad_Value`) 0.0 0.15)
    (goto _label_2)))

(event `Key|Add`
  (params (Key :type "Key Structure"))
  (:`Pressed`
    (set `self.SplinePointNum` (+ (`self.SplinePointNum`) 1))
    (`KismetSystemLibrary.PrintString` (`KismetStringLibrary.Concat_StrStr` "Spline_Num:" (`KismetStringLibrary.Conv_IntToString` (`self.SplinePointNum`))) :!label _label_3)))

(event `Key|Subtract`
  (params (Key :type "Key Structure"))
  (:`Pressed`
    (set `self.SplinePointNum` (- (`self.SplinePointNum`) 1))
    (goto _label_3)))

(event `self.ReceiveBeginPlay`)

(event `EnhancedInput|/Game/Input/inputs/ButtonLeft`
  (params (ActionValue :type Boolean) (ElapsedSeconds :type "Float (double-precision)") (TriggeredSeconds :type "Float (double-precision)") (InputAction :type "InputAction Object Reference" :default "/Game/Input/inputs/ButtonLeft.ButtonLeft"))
  ;[1 1 1] Comment
  (:`Triggered`
    (`self.AddMovementInput` (0.0 -5.0 0.0) :!label _label_4)))

(event `EnhancedInput|/Game/Input/inputs/ButtonRight`
  (params (ActionValue :type Boolean) (ElapsedSeconds :type "Float (double-precision)") (TriggeredSeconds :type "Float (double-precision)") (InputAction :type "InputAction Object Reference" :default "/Game/Input/inputs/ButtonRight.ButtonRight"))
  ;[1 1 1] Comment
  (:`Triggered`
    (`self.AddMovementInput` (0.0 5.0 0.0) :!label _label_5)))

(event `EnhancedInput|/Game/Input/inputs/Button1`
  (params (ActionValue :type Boolean) (ElapsedSeconds :type "Float (double-precision)") (TriggeredSeconds :type "Float (double-precision)") (InputAction :type "InputAction Object Reference" :default "/Game/Input/inputs/Button1.Button1"))
  ;[1 1 1] Comment
)

(event `EnhancedInput|/Game/Input/inputs/Button3`
  (params (ActionValue :type Boolean) (ElapsedSeconds :type "Float (double-precision)") (TriggeredSeconds :type "Float (double-precision)") (InputAction :type "InputAction Object Reference" :default "/Game/Input/inputs/Button3.Button3"))
  ;[1 1 1] Comment
)

(event `DpadLeft`
  ;[1 1 1] Comment
  (if (`KismetMathLibrary.NearlyEqual_FloatFloat` (`self.Dpad_Value`) 0.85 0.15)
    (goto _label_4)))

(event `DpadRight`
  ;[1 1 1] Comment
  (if (`KismetMathLibrary.NearlyEqual_FloatFloat` (`self.Dpad_Value`) 0.28 0.15)
    (goto _label_5)))

(event `Key|Two`
  (params (Key :type "Key Structure"))
  (:`Pressed`
    (`PlayerController.SetViewTargetWithBlend` (`GameplayStatics.GetPlayerController` 0) (`ActorComponent.GetOwner` (`self.Camera`)) 0.0 "VTBlend_Linear" 0.0 false)))

(event `self.ReceiveTick`
  (params (DeltaSeconds :type "Float (single-precision)"))
  (`self.Update_Movement`)
  (`self.Check_Dpad_Zero`))

(event `EnhancedInput|/Game/Input/inputs/ButtonDown`
  (params (ActionValue :type Boolean) (ElapsedSeconds :type "Float (double-precision)") (TriggeredSeconds :type "Float (double-precision)") (InputAction :type "InputAction Object Reference" :default "/Game/Input/inputs/ButtonDown.ButtonDown"))
  ;[1 1 1] Comment
  (:`Triggered`
    (`self.AddMovementInput` (-5.0 0.0 0.0) :!label _label_6)))

(event `Key|PageUp`
  (params (Key :type "Key Structure"))
  (:`Pressed`
    (set `self.Esteira_control` 1.0)
    (`KismetSystemLibrary.PrintString` (`KismetStringLibrary.Concat_StrStr` "PgUp:" (`KismetStringLibrary.Conv_DoubleToString` (`self.Esteira_control`))) :!label _label_7))
  (:`Released`
    (set `self.Esteira_control` 0.0 :!label _label_8)
    (goto _label_7)))

(event `EnhancedInput|/Game/Input/inputs/Button2`
  (params (ActionValue :type Boolean) (ElapsedSeconds :type "Float (double-precision)") (TriggeredSeconds :type "Float (double-precision)") (InputAction :type "InputAction Object Reference" :default "/Game/Input/inputs/Button2.Button2"))
  ;[1 1 1] Comment
  (:`Triggered`
    (`self.Jump`)))

(event `EnhancedInput|/Game/Input/inputs/Button4`
  (params (ActionValue :type Boolean) (ElapsedSeconds :type "Float (double-precision)") (TriggeredSeconds :type "Float (double-precision)") (InputAction :type "InputAction Object Reference" :default "/Game/Input/inputs/Button4.Button4")))

(event `DpadDown`
  ;[1 1 1] Comment
  (if (`KismetMathLibrary.NearlyEqual_FloatFloat` (`self.Dpad_Value`) 0.57 0.15)
    (goto _label_6)))

(event `Key|PageDown`
  (params (Key :type "Key Structure"))
  (:`Pressed`
    (set `self.Esteira_control` -1.0)
    (goto _label_7))
  (:`Released`
    (goto _label_8)))

(event `EnhancedInput|/Game/Input/inputs/LeftY`
  (params (ActionValue :type "Float (double-precision)") (ElapsedSeconds :type "Float (double-precision)") (TriggeredSeconds :type "Float (double-precision)") (InputAction :type "InputAction Object Reference" :default "/Game/Input/inputs/LeftY.LeftY"))
  ;[1 1 1] Comment
  (:`Triggered`
    (set `self.LeftY_Value` ActionValue)))

(event `Update_Movement`
  (bind _leftx_value (`self.LeftX_Value`))
  (bind _lefty_value (`self.LeftY_Value`))
  ;[1 1 1] Comment
  (`|ExecutionSequence`
    (:`then_0`
      (`|ExecutionSequence`
        (:`then_0`
          (if (<= _lefty_value 0.25)
            (`self.AddMovementInput` (5.0 0.0 0.0))))
        (:`then_1`
          (if (>= _lefty_value 0.75)
            (`self.AddMovementInput` (-5.0 0.0 0.0))))))
    (:`then_1`
      (`|ExecutionSequence`
        (:`then_0`
          (if (<= _leftx_value 0.25)
            (`self.AddMovementInput` (0.0 -5.0 0.0))))
        (:`then_1`
          (if (>= _leftx_value 0.75)
            (`self.AddMovementInput` (-0.0 5.0 0.0))))))))

(event `EnhancedInput|/Game/Input/inputs/LeftX`
  (params (ActionValue :type "Float (double-precision)") (ElapsedSeconds :type "Float (double-precision)") (TriggeredSeconds :type "Float (double-precision)") (InputAction :type "InputAction Object Reference" :default "/Game/Input/inputs/LeftX.LeftX"))
  ;[1 1 1] Comment
  (:`Triggered`
    (set `self.LeftX_Value` ActionValue)))

(fn `UserConstructionScript`)